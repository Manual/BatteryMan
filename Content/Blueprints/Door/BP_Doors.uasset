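; BP_Doors is a door that opens once all linked pressure-plate Platforms are pressed, and ignores releases once opening or opened.
; BeginPlay binds plate events to a pressed counter that drives a Closed/Opening/Opened/Closing state.
; Tick animates the door by scaling its Z over MovementTimeSeconds, disabling itself when movement ends.
; The first opening also spawns a hanging flag tagged "DLF" at a hard-coded transform.
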(event `self.ReceiveTick`
  (params (DeltaSeconds :type "Float (single-precision)"))
  (bind (_relativescale3d_x _relativescale3d_y _relativescale3d_z) (`KismetMathLibrary.BreakVector` (`SceneComponent.RelativeScale3D` (`self.Door`))))
  (switch `/Game/Blueprints/Door/DoorState` (`self.CurrentState`)
    (:`NewEnumerator0`
      (`self.SetActorTickEnabled` false :!label _label))
    (:`NewEnumerator1`
      (`SceneComponent.SetRelativeScale3D` (`self.Door`) (`KismetMathLibrary.MakeVector` _relativescale3d_x _relativescale3d_y (`KismetMathLibrary.FClamp` (+ (`self.GetMovementAmount` DeltaSeconds) _relativescale3d_z) (`self.OpenedScaleZ`) (`self.ClosedScaleZ`))) :!label _label_2)
      (`self.EndMovementIfDone`))
    (:`NewEnumerator2`
      (goto _label))
    (:`NewEnumerator3`
      (goto _label_2))))

(event `self.ReceiveBeginPlay`
  (for _array_element (`self.Platforms`)
    (add `/Game/Blueprints/Door/BP_PressurePlate.Pressed` _array_element (delegate `OnPressed`))
    (add `/Game/Blueprints/Door/BP_PressurePlate.Released` _array_element (delegate `OnReleasedPressure`))))

(event `OnPressed`
  (bind _result (`/Engine/EditorBlueprintResources/StandardMacros.IncrementInt` (`self.PressedPlates`))
    (:`  `
      (`KismetSystemLibrary.PrintString` (`KismetStringLibrary.Conv_IntToString` _result))
      (if (== _result (`KismetArrayLibrary.Array_Length` (`self.Platforms`)))
        (`self.ToggleState` "NewEnumerator3")
        (`/Engine/EditorBlueprintResources/StandardMacros.DoOnce` false
          (:`Completed`
            (bind _returnvalue (`|SpawnActorFromClass` "/Game/SM_HangingFlag_03_Blueprint.SM_HangingFlag_03_Blueprint_C" (`KismetMathLibrary.MakeTransform` (2707.0 427.0 130.0) (struct :`Roll` -90.0)) "Undefined" "OverrideRootScale" null null))
            (`KismetArrayLibrary.Array_Add` (`Actor.Tags` _returnvalue) "DLF")))))))

(event `OnReleasedPressure`
  (bind _currentstate (`self.CurrentState`))
  (if (not (or (`|EnumEquality` _currentstate "NewEnumerator3") (`|EnumEquality` _currentstate "NewEnumerator2")))
    (`/Engine/EditorBlueprintResources/StandardMacros.DecrementInt` (`self.PressedPlates`)
      (:`  `
        (`self.ToggleState` "NewEnumerator1")))))

(fn `EndMovementIfDone`
  (bind (_relativescale3d_x _relativescale3d_y _relativescale3d_z) (`KismetMathLibrary.BreakVector` (`SceneComponent.RelativeScale3D` (`self.Door`))))
  (switch `/Game/Blueprints/Door/DoorState` (`self.CurrentState`)
    (:`NewEnumerator1`
      (if (`KismetMathLibrary.NearlyEqual_FloatFloat` (`self.ClosedScaleZ`) _relativescale3d_z)
        (set `self.CurrentState` "NewEnumerator0")))
    (:`NewEnumerator3`
      (if (`KismetMathLibrary.NearlyEqual_FloatFloat` (`self.OpenedScaleZ`) _relativescale3d_z)
        (set `self.CurrentState` "NewEnumerator2")))))

(fn `GetMovementAmount`
  (params (DeltaTime :type "Float (double-precision)"))
  (returns (MovementAmount :type "Float (double-precision)"))
  (bind _returnvalue (* DeltaTime (`self.ClosedScaleZ`) (/ 1.0 (`self.MovementTimeSeconds`))))
  (switch `/Game/Blueprints/Door/DoorState` (`self.CurrentState`)
    (:`NewEnumerator0`
      _)
    (:`NewEnumerator1`
      (return _returnvalue))
    (:`NewEnumerator2`
      _)
    (:`NewEnumerator3`
      (return (* _returnvalue -1.0))))
  (return 0.0))

(fn `ToggleState`
  (params (Selection :type "/Game/Blueprints/Door/DoorState Enum" :default "NewEnumerator0"))
  (set `self.CurrentState` Selection)
  (`self.SetActorTickEnabled` true))

(fn `UserConstructionScript`
  (bind (_relativescale3d_x _relativescale3d_y _relativescale3d_z) (`KismetMathLibrary.BreakVector` (`SceneComponent.RelativeScale3D` (`self.Door`))))
  ;[1 1 1] Door Open/Closed State
  (set `self.ClosedScaleZ` _relativescale3d_z)
  (if (`self.bStartsOpened`)
    (`SceneComponent.SetRelativeScale3D` (`self.Door`) (`KismetMathLibrary.MakeVector` _relativescale3d_x _relativescale3d_y (`self.OpenedScaleZ`)))
    (set `self.CurrentState` "NewEnumerator2")))